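; Spawner actor that creates a copy of ObjectToSpawn's class at its transform with a sound, and respawns it over time.
; BeginPlay plays a fire effect, then makes the first spawn after an initial delay.
; A player or enemy leaving the sphere clears SpawnedSmth, which is treated as a pickup.
; Tick polls that flag and respawns through a Delay of SpawnTimer.
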(event `self.ReceiveTick`
  (params (DeltaSeconds :type "Float (single-precision)"))
  ;[1 1 1] Spawn Items
  (if (and (`self.FirstSpawn`) (not (`self.SpawnedSmth`)))
    (`KismetSystemLibrary.Delay` (`self.SpawnTimer`))
    (`self.SpawnFromClass`)))

(event `self.ReceiveBeginPlay`
  ;[1 1 1] First Spawn
  (`GameplayStatics.SpawnEmitterAtLocation` "/Game/StarterContent/Particles/P_Fire.P_Fire" (`self.K2_GetActorLocation`))
  (`KismetSystemLibrary.Delay` (`self.TimeUnderFirstSpawn`))
  (`self.SpawnFromClass`)
  (set `self.FirstSpawn` true))

(event `self.Sphere1.OnComponentEndOverlap`
  (params (OverlappedComponent :type "PrimitiveComponent Object Reference") (OtherActor :type "Actor Object Reference") (OtherComp :type "PrimitiveComponent Object Reference") (OtherBodyIndex :type Integer))
  ;[1 1 1] Picked up by someone
  (`|ExecutionSequence`
    (:`then_0`
      (cast `/Game/Logic/Blueprints/Character/Player/BP_Player` OtherActor)
      (set `self.SpawnedSmth` false))
    (:`then_1`
      (cast `/Game/Logic/Blueprints/Character/AI/BP_Enemy` OtherActor)
      (set `self.SpawnedSmth` false))))

(fn `SpawnFromClass`
  (`|SpawnActorFromClass` (`GameplayStatics.GetObjectClass` (`self.ObjectToSpawn`)) (`self.GetTransform` self) "Undefined" "OverrideRootScale" null null)
  (`GameplayStatics.PlaySound2D` "/Game/Sounds/SpawnItem.SpawnItem" 1.0 1.0 0.0 null null)
  (set `self.SpawnedSmth` true))

(fn `UserConstructionScript`)