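; BP_Enemy is an AI-controlled armed enemy that shoots, reloads, dies and respawns.
; It takes its weapon from a child actor, spawns projectiles near the hand socket along its camera's view, and refills ammo from an AK reserve.
; Tick refreshes a random strafe value on a delay and triggers Death at zero health.
; Death stops the controller's brain logic and destroys the actor, whose Destroyed event asks ThirdPersonGameMode to respawn AI.
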(event `self.ReceiveBeginPlay`
  ;[1 1 1] WeaponReference
  (`self.Get_Weapon`))

(event `self.ReceiveTick`
  (params (DeltaSeconds :type "Float (single-precision)"))
  (if (<= (`self.Health`) 0)
    (`/Engine/EditorBlueprintResources/StandardMacros.DoOnce` false
      (:`Completed`
        (`self.Death`)))
    (else
      ;[1 1 1] Change Vector of Strafe
      (`KismetSystemLibrary.Delay` 3.0)
      (set `self.RandomFloat` (`KismetMathLibrary.RandomFloatInRange` -1.0 1.0)))))

(event `Death`
  ;[1 1 1] Death event
  (set `self.IsDead` true)
  (`GameplayStatics.PlaySound2D` "/Game/Sounds/YesIAm.YesIAm" 1.0 1.0 0.0 null null)
  (bind _asbp_aicontroller (cast `/Game/Logic/Blueprints/Character/AI/BP_AIController` (`AIBlueprintHelperLibrary.GetAIController` self)))
  (`BrainComponent.StopLogic` (`AIController.BrainComponent` _asbp_aicontroller) "")
  (`KismetSystemLibrary.Delay` 2.0)
  (`self.K2_DestroyActor`))

(event `self.ReceiveDestroyed`
  ;[1 1 1] Respawn event
  (bind _asthird_person_game_mode (cast `/Game/Logic/Blueprints/ThirdPersonGameMode` (`GameplayStatics.GetGameMode`)))
  (`/Game/Logic/Blueprints/ThirdPersonGameMode.RespawnAI` _asthird_person_game_mode))

(fn `FindTrace`
  (returns (NewParam :type "Transform Structure"))
  (bind _skeletalmesh (`/Game/Logic/Blueprints/Weapon/BP_Weapon.SkeletalMesh` (`self.WeaponReference`)))
  (bind _returnvalue_location (`KismetMathLibrary.BreakTransform` (`SceneComponent.GetSocketTransform` _skeletalmesh (`SkinnedMeshComponent.GetSocketBoneName` _skeletalmesh "Hand_Socket") "RTS_World")))
  (bind _desiredview (`CameraComponent.GetCameraView` (`self.Camera`) 0.0))
  (return (`KismetMathLibrary.MakeTransform` (+ _returnvalue_location (* (`KismetMathLibrary.GetForwardVector` (`.Rotation` (break `MinimalViewInfo` _desiredview))) 100.0)) (`.Rotation` (break `MinimalViewInfo` _desiredview)))))

(fn `OpenFire`
  (if (> (`/Game/Logic/Blueprints/Weapon/BP_Weapon.Ammo` (`self.WeaponReference`)) 0)
    (bind _newparam (`self.FindTrace`))
    (`|SpawnActorFromClass` "/Game/Logic/Blueprints/Weapon/BP_Projectile.BP_Projectile_C" _newparam "Undefined" "OverrideRootScale" null null)
    (`/Engine/EditorBlueprintResources/StandardMacros.DecrementInt` (`/Game/Logic/Blueprints/Weapon/BP_Weapon.Ammo` (`self.WeaponReference`))
      (:`  `
        (`GameplayStatics.PlaySound2D` "/Game/Sounds/Piu.Piu" 1.0 1.0 0.0 null null)))))

(fn `Reload`
  (bind _weaponreference (`self.WeaponReference`))
  (bind _weaponreference_2 (`self.WeaponReference`))
  (bind _weaponreference_3 (`self.WeaponReference`))
  (bind _needestammo (`self.NeedestAmmo`))
  (if (not (or (== (`/Game/Logic/Blueprints/Weapon/BP_Weapon.Ammo` (`self.WeaponReference`)) 30) (== (`self.AmmoForAK`) 0)))
    (set `self.OnReload` true)
    (bind _output_get (set `self.NeedestAmmo` (- (`/Game/Logic/Blueprints/Weapon/BP_Weapon.Magazine` _weaponreference_2) (`/Game/Logic/Blueprints/Weapon/BP_Weapon.Ammo` _weaponreference_2))))
    (if (> (`self.AmmoForAK`) _output_get)
      (set `/Game/Logic/Blueprints/Weapon/BP_Weapon.Ammo` (+ (`/Game/Logic/Blueprints/Weapon/BP_Weapon.Ammo` _weaponreference) _needestammo) _weaponreference)
      (set `self.AmmoForAK` (- (`self.AmmoForAK`) _needestammo))
      (else
        (set `/Game/Logic/Blueprints/Weapon/BP_Weapon.Ammo` (+ (`/Game/Logic/Blueprints/Weapon/BP_Weapon.Ammo` _weaponreference_3) (`self.AmmoForAK`)) _weaponreference_3)
        (set `self.AmmoForAK` 0)))))

(fn `UserConstructionScript`)