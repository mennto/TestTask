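; Pickup actor that grants AK ammunition to whoever touches it, either the player or an enemy AI.
; On overlap with the static mesh, it casts the other actor to BP_Player and BP_Enemy in sequence and adds its Value to that character's AmmoForAK.
; It then destroys itself, playing a 2D pickup sound only when the player collects it.
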(event `self.StaticMesh.OnComponentBeginOverlap`
  (params (OverlappedComponent :type "PrimitiveComponent Object Reference") (OtherActor :type "Actor Object Reference") (OtherComp :type "PrimitiveComponent Object Reference") (OtherBodyIndex :type Integer) (bFromSweep :type Boolean) (SweepResult :type "HitResult Structure (by ref)"))
  (`|ExecutionSequence`
    (:`then_0`
      ;[1 1 1] Picked by Player
      (bind _asbp_player (cast `/Game/Logic/Blueprints/Character/Player/BP_Player` OtherActor))
      (set `/Game/Logic/Blueprints/Character/Player/BP_Player.AmmoForAK` (+ (`/Game/Logic/Blueprints/Character/Player/BP_Player.AmmoForAK` _asbp_player) (`self.Value`)) _asbp_player)
      (`GameplayStatics.PlaySound2D` "/Game/Sounds/ItsForMe.ItsForMe" 1.0 1.0 0.0 null null)
      (`self.K2_DestroyActor`))
    (:`then_1`
      ;[1 1 1] Picked by AI
      (bind _asbp_enemy (cast `/Game/Logic/Blueprints/Character/AI/BP_Enemy` OtherActor))
      (set `/Game/Logic/Blueprints/Character/AI/BP_Enemy.AmmoForAK` (+ (`/Game/Logic/Blueprints/Character/AI/BP_Enemy.AmmoForAK` _asbp_enemy) (`self.Value`)) _asbp_enemy)
      (`self.K2_DestroyActor`))))

(fn `UserConstructionScript`)